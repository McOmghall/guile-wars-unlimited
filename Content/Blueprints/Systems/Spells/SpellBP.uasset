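; SpellBP is a base spell actor exposing overridable hooks for before shooting, shooting, after shooting and failure.
; On BeginPlay it can override its follower component's offset, then runs the pre-shot hook.
; Mana consumption and readiness propagate through calls, while a status enum records whether the spell was ready when launched.
; Shooting sets a limited lifespan and destroys sounds spawned by child sound-effect manager components.
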(event Custom|BeforeShooting)

(event Custom|ConsumeMana
  (Default|CallConsumeManaPropagate))

(event Custom|SpellReady
  (Default|CallSpellReadyPropagate)
  (Variables|SpellInternals|SetSpellStatus "NewEnumerator1"))

(event Custom|Shoot
  (params (Target :type Targetable%20BP%20Interface%20Interface) (ScaleVelocity :type Vector))
  (CallFunction|AfterShooting)
  (Actor|SetLifeSpan 1e+01)
  (for _array_element (Components|GetChildrenComponents (Variables|Default|GetDefaultSceneRoot) true) ; Destroy all spawned sounds,\nif they exist
    (bind _assound_effects_manager_cbp (Utilities|Casting|CastToSoundEffectsManagerCBP _array_element))
    (Default|DestroyAllSpawnedSounds _assound_effects_manager_cbp)))

(event Custom|AfterShooting
  (switch Utilities|FlowControl|Switch|SwitchonSpellStatusEnumBP (Variables|SpellInternals|GetSpellStatus)
    (:NewEnumerator0
      (Variables|SpellInternals|SetSpellStatus "NewEnumerator2"))
    (:NewEnumerator1
      (Variables|SpellInternals|SetSpellStatus "NewEnumerator3"))))

(event Custom|SpellFailed)

(event EventBeginPlay
  (if (Variables|Positioning|GetOverrideOffset)
    (Variables|/Game/Blueprints/Systems/CharacterAttributes/FollowerCBP.FollowerCBP_C|SetOffset (Variables|Default|GetFollowerCBP) (Variables|Positioning|GetOffsetOverride)))
  (CallFunction|BeforeShooting))

(fn ConstructionScript)