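; Spell projectile that follows its shooter until fired, then flies at a target and spawns an explosion on first overlap.
; Swaps blocking collision for magic collision on Shoot and detaches its follower component.
; Aims by scaling target-relative axes, slowed unless the spell is ready, and homes using target acceleration times its own multiplier.
; Impact destroys the projectile, choosing the explosion class by spell status with a default fallback.
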(event OnComponentBeginOverlap(MagicProjectileCollision)
  (params (OverlappedComponent :type Primitive%20Component%20Object%20Reference) (OtherActor :type Actor%20Object%20Reference) (OtherComp :type Primitive%20Component%20Object%20Reference) (OtherBodyIndex :type Integer) (bFromSweep :type Boolean) (SweepResult :type Hit%20Result%20Structure%20%28by%20ref%29))
  (bind _explosionperstateoverride (Variables|Default|GetExplosionPerStateOverride))
  (bind _spellstatus (Variables|Default|GetSpellStatus))
  (bind (_value _returnvalue) (Utilities|Map|Find _explosionperstateoverride _spellstatus))
  (Utilities|FlowControl|DoOnce false
    (:Completed
      (Game|SpawnActorfromClass (select _returnvalue _value (Variables|Default|GetExplosionAtImpactDefault)) (Transformation|GetActorTransform) "AlwaysSpawn" 0 (Game|GetInstigator))
      (Actor|DestroyActor))))

(event EventConsumeMana
  (|CallParentFunction))

(event EventSpellReady
  (|CallParentFunction))

(event EventAfterShooting
  (|CallParentFunction))

(event EventShoot
  (params (Target :type Targetable%20BP%20Interface%20Interface) (ScaleVelocity :type Vector))
  (bind _returnvalue (Math|Vector|Normalize ScaleVelocity))
  (bind _returnvalue_2 (* _returnvalue 2e+02))
  (CallFunction|DeactivateFollower) ; Stop Following movement of shooter
  (CallFunction|SwapCollisions (Variables|Default|GetBlockingCollision) (Variables|Default|GetMagicProjectileCollision)) ; Activate magic
  (CallFunction|SetTarget (Variables|Default|GetProjectileMovement) Target (Utilities|Select :Index (Variables|Default|GetSpellStatus) :NewEnumerator0 _returnvalue_2 :NewEnumerator1 ScaleVelocity :NewEnumerator2 _returnvalue_2 :NewEnumerator3 _returnvalue_2)) ; Take Aim and Fire
  (|CallParentFunction Target ScaleVelocity))

(event EventBeforeShooting
  (|CallParentFunction)
  (CallFunction|SwapCollisions (Variables|Default|GetMagicProjectileCollision) (Variables|Default|GetBlockingCollision)) ; Block all\nDon't activate magic
)

(fn ConstructionScript)

(fn DeactivateFollower
  (bind _followercbp (Variables|Default|GetFollowerCBP)
    (:then
      (Variables|/Game/Blueprints/Systems/Spells/Plumbing/FollowerCBP.FollowerCBP_C|SetApplyOffset _followercbp false)
      (Components|Activation|Deactivate _followercbp)
      (Components|DestroyComponent _followercbp))
    (:else)))

(fn SetTarget
  (params (ProjectileMovementComponent :type Projectile%20Movement%20Component%20Object%20Reference) (Target :type Targetable%20BP%20Interface%20Interface) (VelocityScale :type Vector))
  (bind (_x _y _z) (Math|Vector|BreakVector VelocityScale))
  (Utilities|IsValid ProjectileMovementComponent ; ProjectileMovement not present?\nBypass the whole function
    (:Is%20Valid
      (Utilities|IsValid (Utilities|ToObject(Interface) Target) ; Target not present?\nJust activate the projectile movement
        (:Is%20Valid
          (bind _location (Default|GetTargetableLocation Target))
          (Variables|/Script/Engine.MovementComponent|SetVelocity ProjectileMovementComponent (+ (* (Math|Vector|Normalize (Math|Vector|GetForwardVector (Math|Rotator|FindLookatRotation (Transformation|GetActorLocation) _location))) _x) (* (Math|Vector|Normalize (Math|Vector|GetRightVector (Math|Rotator|FindLookatRotation (Transformation|GetActorLocation) _location))) _y) (* (Math|Vector|Normalize (Math|Vector|GetUpVector (Math|Rotator|FindLookatRotation (Transformation|GetActorLocation) _location))) _z))) ; Set velocity of projectile
          (bind (_hometo _homingaccelmag) (Default|GetHomingComponent Target))
          (Variables|/Script/Engine.ProjectileMovementComponent|SetHomingTargetComponent ProjectileMovementComponent _hometo) ; Home In objective by a factor\ngiven by both objective and projectile
          (Variables|/Script/Engine.ProjectileMovementComponent|SetHomingAccelerationMagnitude ProjectileMovementComponent (* _homingaccelmag (Variables|Default|GetHomingAccelMagMultiplier))))
        (:Is%20Not%20Valid
          _))
      (Components|Activation|Activate ProjectileMovementComponent true) ; Fire!
    )
    (:Is%20Not%20Valid
      _))
  (return ProjectileMovementComponent))

(fn DrawDebugTrajectory
  (bind _returnvalue (Transformation|GetActorLocation))
  (Rendering|Debug|DrawDebugLine _returnvalue (+ _returnvalue (* (Transformation|GetVelocity) -1)) (Math|Conversions|ToLinearColor(Vector) (Math|Random|RandomUnitVector)) 1.0 1.0))

(fn DrawDebugDivergence
  (params (Origin :type Vector) (Movement1 :type Vector) (Movement2 :type Vector))
  (Rendering|Debug|DrawDebugLine Origin (+ Origin Movement1) "(R=1.000000,G=0.000000,B=0.000000,A=1.000000)" 1.0 2.0)
  (Rendering|Debug|DrawDebugLine Origin (+ Origin Movement2) "(R=0.000000,G=0.000000,B=1.000000,A=1.000000)" 1.0 2.0))

(fn SwapCollisions
  (params (out :type Sphere%20Component%20Object%20Reference) (In :type Primitive%20Component%20Object%20Reference))
  (Components|Activation|Deactivate out)
  (Collision|SetCollisionEnabled out "NoCollision")
  (Components|Activation|Activate In true)
  (Collision|SetCollisionEnabled In "QueryAndPhysics"))