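; Magic Missile spell projectile Blueprint that specializes the firing behavior of its parent projectile class.
; On Shoot it waits for a custom delay, then plays the magic missile sound through the instigator's sound effects manager.
; It then calls the parent Shoot with the same target and a distortion initial velocity added to the velocity scale.
; BeginPlay and construction only call the parent.
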(event EventBeginPlay
  (|CallParentFunction))

(event EventShoot
  (params (Target :type Targetable%20BP%20Interface%20Interface) (ScaleVelocity :type Vector))
  (Utilities|FlowControl|Delay (Variables|Default|GetCustomDelay))
  (Default|PlaySound (Variables|Default|GetDelegateToInstigatorSoundEffectsManagerBP) "/Game/SFX/SFX_MagicMissile.SFX_MagicMissile")
  (|CallParentFunction Target (+ ScaleVelocity (Variables|Default|GetDistortionInitialVelocity))))

(fn ConstructionScript
  (|CallParentFunction))