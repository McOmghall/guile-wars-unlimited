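; Circle of fire spell actor that deals damage over time to player characters touching its ring.
; The construction script spaces sphere colliders and fire particle emitters around a configurable radius by rotating an offset vector.
; Each tick, a macro scans every collider for overlapping MainPlayerBP actors implementing DamageableBPInterface and sends them DamagePerSecond scaled by delta time, once per overlapped collider.
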(event EventTick
  (params (DeltaSeconds :type Float%20%28single-precision%29))
  (bind _actor (Utilities|ForAllActorsTouchingtheCircle)
    (:Exec
      (Class|DamageableBPInterface|ReceiveDamage(Message) _actor (* DeltaSeconds (Variables|SpellConfig|GetDamagePerSecond))))))

(fn ConstructionScript
  (bind _colliderscount (Variables|CircleConfig|GetCollidersCount))
  (for _index (range 0 _colliderscount) ; Create a circle of CollidersCount colliders
    (Utilities|FlowControl|Sequence
      (:then_0
        (bind _returnvalue (AddComponent|AddSphereComponent false (Math|Transform|MakeTransform (Math|Vector|RotateVectorAroundAxis (Math|Vector|MakeVector (Variables|CircleConfig|GetCircleRadius) 0.0 0.0) (* _index (/ 3.6e+02 (Math|Conversions|ToFloat(Integer) _colliderscount))) "0, 0,1.000000") "0, 0, 0" "1,1,1"))) ; Create Collision
        (Collision|SetCollisionProfileName _returnvalue (Variables|CircleConfig|GetCollisionProfileName) :!class /Script/Engine.PrimitiveComponent)
        (Components|Sphere|SetSphereRadius _returnvalue (Variables|CircleConfig|GetCollidersRadius) true)
        (Utilities|Array|Add (Variables|CircleConfig|GetAllColliders) _returnvalue))
      (:then_1
        (bind _returnvalue_2 (AddComponent|AddParticleSystemComponent false (Math|Transform|MakeTransform (Math|Vector|RotateVectorAroundAxis (Math|Vector|MakeVector (Variables|CircleConfig|GetCircleRadius) 0.0 0.0) (* _index (/ 3.6e+02 (Math|Conversions|ToFloat(Integer) _colliderscount))) "0, 0,1.000000") "0, 0, 0" "1,1,1")))
        (Effects|Components|ParticleSystem|SetTemplate _returnvalue_2 (Variables|CircleConfig|GetFireParticles))))))