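; Spell Blueprint that spawns a fan of magic missile projectiles at the instigator and fires them at a target.
; The SpawnMissiles timeline starts before shooting, spawning missiles through Spawn events and triggering mana consumption and spell readiness.
; Each missile gets an index-based delay, plus offset and initial velocity rotated across a centered TotalAngle arc.
; Shoot stores target and velocity scale, fires existing missiles, and later spawns fire immediately.
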(event EventAfterShooting
  (|CallParentFunction))

(event EventBeginPlay
  (|CallParentFunction))

(event EventConsumeMana
  (|CallParentFunction))

(event EventSpellReady
  (|CallParentFunction))

(event EventShoot
  (params (Target :type Targetable%20BP%20Interface%20Interface) (ScaleVelocity :type Vector))
  (Variables|Default|SetScaleVelocity ScaleVelocity)
  (Variables|Default|SetTarget Target)
  (Variables|Default|SetShot? true)
  (|CallParentFunction Target ScaleVelocity)
  (for _array_element (Variables|Default|GetChildrenMissiles)
    (Utilities|IsValid _array_element
      (:Is%20Valid
        (Default|Shoot _array_element Target ScaleVelocity)))))

(event EventBeforeShooting
  (bind _returnvalue (Game|GetInstigator))
  (bind _currentmissile (Variables|Default|GetCurrentMissile))
  (|CallParentFunction)
  (Timeline|SpawnMissiles Play
    (:Spawn
      (Utilities|FlowControl|Sequence
        (:then_0
          (bind _returnvalue_2 (Game|SpawnActorfromClass "/Game/Blueprints/Systems/Spells/SpellProjectileMagicMissileBP.SpellProjectileMagicMissileBP_C" (Transformation|GetActorTransform _returnvalue) "AlwaysSpawn" 0 (* _currentmissile 0.1) (CallFunction|OffsetForwardsOfMissile "500.000000, 0, 0" _currentmissile) true (CallFunction|OffsetUpwardsOfMissile "0, 0,100.000000" _currentmissile) _returnvalue)) ; Start Spell
          (Utilities|IsValid _returnvalue_2
            (:Is%20Valid
              (Default|SpellReady _returnvalue_2)
              (if (Variables|Default|GetShot?)
                (Default|Shoot _returnvalue_2 (Variables|Default|GetTarget) (Variables|Default|GetScaleVelocity)))
              (Utilities|Array|Add (Variables|Default|GetChildrenMissiles) _returnvalue_2))))
        (:then_1
          (Math|Integer|IncrementInt _currentmissile))))
    (:ConsumeMana
      (CallFunction|ConsumeMana)
      (CallFunction|SpellReady))))

(fn ConstructionScript)

(fn AngleOfMissile
  (params (Index :type Integer))
  (bind _totalangle (Variables|Default|GetTotalAngle))
  (return (- (* Index (/ _totalangle (Math|Conversions|ToFloat(Integer) (Math|Integer|Max(Integer) (- (Variables|Default|GetAmountOfMissiles) 1) 1)))) (/ _totalangle 2.0))))

(fn OffsetUpwardsOfMissile
  (params (OffsetAtCenter :type Vector) (Index :type Integer))
  (return (Math|Vector|RotateVectorAroundAxis OffsetAtCenter (CallFunction|AngleOfMissile Index) "1.000000, 0, 0")))

(fn OffsetForwardsOfMissile
  (params (OffsetAtCenter :type Vector) (Index :type Integer))
  (return (Math|Vector|RotateVectorAroundAxis OffsetAtCenter (CallFunction|AngleOfMissile Index) "0.000000, 0,1.000000")))