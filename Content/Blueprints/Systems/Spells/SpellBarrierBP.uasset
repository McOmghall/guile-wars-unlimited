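; Barrier spell actor that nullifies damage taken by its instigator and turns part of it into mana.
; On BeginPlay it caches the instigator's mana and health manager components, binds to the damage-received event, and calls ConsumeMana after a brief delay.
; Rather than intercepting hits, it reacts to each damage event by earning the amount back as health and granting mana scaled by ProportionOfDamageAsMana.
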(event Custom|NullifyDamage
  (params (DamageReceived :type Float%20%28single-precision%29) (MaxHealth :type Float%20%28single-precision%29) (CurrentHealth :type Float%20%28single-precision%29) (WillDie :type Boolean))
  (Default|Earn (Variables|Default|GetHealthManager) DamageReceived)
  (Default|Earn (Variables|Default|GetManaManager) (* DamageReceived (Variables|Default|GetProportionOfDamageAsMana))))

(event EventBeginPlay
  (bind _returnvalue (Game|GetInstigator))
  (bind _returnvalue_2 (Actor|GetComponentbyClass _returnvalue "/Game/Blueprints/Systems/CharacterAttributes/HealthManagerCBP.HealthManagerCBP_C"))
  (|CallParentFunction)
  (Utilities|FlowControl|Sequence
    (:then_0
      (Variables|Default|SetManaManager (Actor|GetComponentbyClass (Game|GetInstigator) "/Game/Blueprints/Systems/CharacterAttributes/ManaManagerCBP.ManaManagerCBP_C")))
    (:then_1
      (bind _output_get (Variables|Default|SetHealthManager _returnvalue_2))
      (Utilities|IsValid _output_get
        (:Is%20Valid
          (EventDispatchers|BindEventtoOnDamageReceived _returnvalue_2 (delegate Custom|NullifyDamage)))))
    (:then_2
      (Utilities|FlowControl|Delay 0.05)
      (CallFunction|ConsumeMana))))

(fn ConstructionScript
  (|CallParentFunction))