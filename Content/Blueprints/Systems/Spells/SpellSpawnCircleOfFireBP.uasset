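; Spell actor that lets the player aim and cast a circle of fire on the floor at the current target.
; It consumes mana shortly after BeginPlay, then until shot shows a FakeCircleOfFireBP preview eased toward the target spot each tick.
; Placement traces from instigator toward target, then straight down to find the floor.
; Shoot spawns the real CircleOfFireBP there and expires both spell and preview.
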(event EventBeginPlay
  (|CallParentFunction)
  (Utilities|FlowControl|Delay 0.05) ; Hack
  (CallFunction|ConsumeMana)
  (Timeline|SpawnCircleOfFireTimeline Play))

(event EventShoot
  (params (Target :type Targetable%20BP%20Interface%20Interface) (ScaleVelocity :type Vector))
  (bind _fakecircle (Variables|Default|GetFakeCircle))
  (|CallParentFunction Target ScaleVelocity)
  (bind _where (Utilities|CanSpawnCircleOfFlames Target)
    (:CanSpawn
      (Utilities|SpawnCircleOfFlames _where "/Game/Blueprints/Systems/Spells/CircleOfFireBP.CircleOfFireBP_C"
        (:Exec
          (Actor|SetLifeSpan 0.1)
          (Utilities|IsValid _fakecircle
            (:Is%20Valid
              (Actor|SetLifeSpan _fakecircle 0.1))))))))

(event EventTick
  (params (DeltaSeconds :type Float%20%28single-precision%29))
  (bind _spellstatus (Variables|Default|GetSpellStatus))
  (|CallParentFunction DeltaSeconds)
  (bind _asmain_player_bp (Utilities|Casting|CastToMainPlayerBP (Game|GetInstigator)))
  (bind _currenttarget (Default|GetCurrentTarget _asmain_player_bp))
  (bind _where (Utilities|CanSpawnCircleOfFlames _currenttarget)
    (:CanSpawn
      (if (or (Utilities|Enum|Equal(Enum) _spellstatus "NewEnumerator0") (Utilities|Enum|Equal(Enum) _spellstatus "NewEnumerator1")) ; If spell was not shot yet:
        (Utilities|IsValid (Variables|Default|GetFakeCircle) ; Spawn targeting help
          (:Is%20Valid
            _)
          (:Is%20Not%20Valid
            (bind _returnvalue (Utilities|SpawnCircleOfFlames _where "/Game/Blueprints/Systems/Spells/FakeCircleOfFireBP.FakeCircleOfFireBP_C")
              (:Exec
                (Variables|Default|SetFakeCircle _returnvalue)))))
        (Transformation|SetActorLocation (Variables|Default|GetFakeCircle) (Math|Vector|Lerp(Vector) (Transformation|GetActorLocation (Variables|Default|GetFakeCircle)) _where 0.5) false true)))))

(fn ConstructionScript
  (|CallParentFunction))