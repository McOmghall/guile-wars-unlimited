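; Spell manager actor that gates and launches one managed spell class for its instigator, enforcing mana cost and cooldown.
; StartSpell checks the mana interface, available mana and a UTC-timestamp cooldown, then spawns the spell and returns a result enum.
; It binds to the spell's events so mana spending and ready notification happen later, the latter cast to MainPlayerBP.
; BeginPlay prints an error if the instigator lacks targeting or mana interfaces.
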(event EventBeginPlay
  (bind _returnvalue (Game|GetInstigator))
  (if (not (Math|Boolean|ANDBoolean (Utilities|IsValid _returnvalue) (Utilities|DoesObjectImplementInterface _returnvalue "/Game/Blueprints/Systems/Interfaces/CanAcquireTargetsBPInterface.CanAcquireTargetsBPInterface_C") (Utilities|DoesObjectImplementInterface _returnvalue "/Game/Blueprints/Systems/Interfaces/UsesManaBPInterface.UsesManaBPInterface_C")))
    (Development|PrintString "ERROR: Not suported instigator, needs to implement CanAcquireTargets, UsesMana interfaces")))

(fn ConstructionScript)

(fn StartSpell
  (bind _returnvalue (Game|GetInstigator))
  (bind _instigator (Variables|Actor|GetInstigator))
  (Utilities|FlowControl|Sequence
    (:then_0
      ;[0 0.2752 0 0.2936] Are you a wizard?
      (if (not (Utilities|DoesObjectImplementInterface _instigator "/Game/Blueprints/Systems/Interfaces/UsesManaBPInterface.UsesManaBPInterface_C"))
        (return "NewEnumerator4" 0)))
    (:then_1
      ;[0 0.2752 0.08257 0.2936] Do we have enough mana?
      (bind _canspendmana (Class|UsesManaBPInterface|CanSpendMana(Message) _instigator (Variables|Default|GetManaCost)))
      (if (not _canspendmana)
        (return "NewEnumerator0" 0)))
    (:then_2
      ;[0 0.2752 0.3119 0.2936] Are we outside CD?
      (if (>= (CallFunction|RemainingCooldown) 0.0)
        (return "NewEnumerator1" 0)))
    (:then_3
      ;[1 0 0 0.5] WE CAN FIRE
      (bind _returnvalue_2 (Game|SpawnActorfromClass (Variables|Default|GetManagedSpellClass) (Transformation|GetActorTransform _returnvalue) "AlwaysSpawn" 0 _returnvalue)) ; Start Spell
      (if (Utilities|IsValid _returnvalue_2)
        (Variables|Default|SetLastLaunched (Math|DateTime|UTCNow))
        (EventDispatchers|BindEventtoConsumeManaPropagate _returnvalue_2 (EventDispatchers|CreateEvent :!event ConsumeMana)) ; Signal Consume mana at appropriate time
        (EventDispatchers|BindEventtoSpellReadyPropagate _returnvalue_2 (EventDispatchers|CreateEvent :!event SpellReady)) ; Signal Spell Ready at appropriate time
      )
      (return (select (Utilities|IsValid _returnvalue_2) "NewEnumerator2" "NewEnumerator3") _returnvalue_2))))

(fn RemainingCooldown
  (return (Math|Timespan|GetTotalSeconds (- (+ (Variables|Default|GetLastLaunched) (Math|Timespan|FromSeconds (Variables|Default|GetCooldown))) (Math|DateTime|UTCNow)))))

(fn ConsumeMana
  (bind _instigator (Variables|Actor|GetInstigator))
  (if (Utilities|DoesObjectImplementInterface _instigator "/Game/Blueprints/Systems/Interfaces/UsesManaBPInterface.UsesManaBPInterface_C")
    (Class|UsesManaBPInterface|SpendMana(Message) _instigator (Variables|Default|GetManaCost))))

(fn SpellReady
  (bind _asmain_player_bp (Utilities|Casting|CastToMainPlayerBP (Variables|Actor|GetInstigator)))
  (Default|SpellReady _asmain_player_bp))