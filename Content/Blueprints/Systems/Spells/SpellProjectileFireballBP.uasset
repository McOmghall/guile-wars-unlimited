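; Fireball spell projectile that layers charge-up visuals and sound onto a parent spell projectile class.
; Before shooting, a timeline animates the mesh's dynamic material shine, triggers mana consumption and, if still in init status, readies the spell.
; Becoming ready swaps startup particles for activated ones and plays the ready sound.
; After shooting, the timeline stops for init, ready and launched-not-ready statuses.
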(event EventAfterShooting
  (|CallParentFunction)
  (switch Utilities|FlowControl|Switch|SwitchonSpellStatusEnumBP (Variables|Default|GetSpellStatus)
    (:NewEnumerator0
      _)
    (:NewEnumerator1
      _)
    (:NewEnumerator2
      _))
  (Audio|Components|Audio|Stop (Variables|Default|GetSpellActivationTimeline)))

(event EventBeginPlay
  (bind _projectilemesh (Variables|Default|GetProjectileMesh))
  (|CallParentFunction)
  (bind _returnvalue (Rendering|Material|CreateDynamicMaterialInstance _projectilemesh 0 (Rendering|Material|GetMaterial _projectilemesh 0) :!class /Script/Engine.PrimitiveComponent))
  (Variables|Default|SetDynamicMaterialFireball _returnvalue))

(event EventConsumeMana
  (|CallParentFunction))

(event EventSpellReady
  (|CallParentFunction)
  (Components|Activation|Deactivate (Variables|Default|GetParticleSystemStartup))
  (Components|Activation|Activate (Variables|Default|GetParticleSystemActivated) false)
  (Default|PlaySoundFireballReady (Variables|Default|GetFireballSoundEffectsManagerCBP)))

(event EventShoot
  (params (Target :type Targetable%20BP%20Interface%20Interface) (ScaleVelocity :type Vector))
  (|CallParentFunction Target ScaleVelocity))

(event EventBeforeShooting
  (|CallParentFunction)
  (Default|PlaySoundFireballStart (Variables|Default|GetFireballSoundEffectsManagerCBP))
  (bind _spellintensity (Timeline|SpellActivationTimeline Play)
    (:Update
      (Rendering|Material|SetScalarParameterValue (Variables|Default|GetDynamicMaterialFireball) "ShineIntensities" _spellintensity :!class /Script/Engine.MaterialInstanceDynamic))
    (:ConsumeMana
      (CallFunction|ConsumeMana))
    (:ActivateSpell
      (switch Utilities|FlowControl|Switch|SwitchonSpellStatusEnumBP (Variables|Default|GetSpellStatus)
        (:NewEnumerator0
          (CallFunction|SpellReady))))))

(fn ConstructionScript)