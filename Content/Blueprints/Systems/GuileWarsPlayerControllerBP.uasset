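; Player controller Blueprint for GuileWars with an unfinished Z-targeting lock-on system.
; While lock-on is active with a valid interface-typed target, Tick calls TurnAtRate on the controlled MyProjectCharacter with a constant rate, ignoring the target's position.
; GetNewTargetByControlMode only clears the target and returns a fixed control mode with targeting off, and GetCurrentTarget is an empty stub.
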(event EventBeginPlay)

(event EventTick
  (params (DeltaSeconds :type Float%20%28single-precision%29))
  (bind _currenttarget (Variables|ZTargeting|GetCurrentTarget))
  ;[1 0.6972 0.6881 0.367] LockOnSystem (Z Targeting)
  (if (and (Variables|ZTargeting|GetbIsLockOnActive) (Utilities|IsValid (Utilities|ToObject(Interface) _currenttarget)))
    (Default|GetasActor _currenttarget)
    (bind _asmy_project_character (Utilities|Casting|CastToMyProjectCharacter (Pawn|GetControlledPawn)))
    (Class|MyProjectCharacter|TurnatRate _asmy_project_character 2e+02)))

(fn ConstructionScript)

(fn GetCurrentTarget
  (return 0))

(fn GetNewTargetbyControlMode
  (params (ControlMode :type ControlModeEnumBP%20Enum :default "NewEnumerator3"))
  (Variables|ZTargeting|SetCurrentTarget 0)
  (return 0 "NewEnumerator3" true false))