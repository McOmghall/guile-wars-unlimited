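; Sound effects component for the fireball spell, with events for the start, ready and not-ready cues.
; Start plays a smoke cue and keeps its handle so Ready can stop it before playing the fireball cue plus a randomly weighted spell-ready sound.
; Not-ready routes a failure sound through the sound effects manager of the owner's instigating player, so it plays from the player rather than this component.
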(event Custom|PlaySoundFireballStart
  (bind _audiocomponent (CallFunction|PlaySound "/Game/SFX/SFX_SmokeFireball_Cue.SFX_SmokeFireball_Cue")))

(event Custom|PlaySoundFireballReady
  (Utilities|IsValid (stale Custom|PlaySoundFireballStart _audiocomponent)
    (:Is%20Valid
      (Audio|Components|Audio|Stop (stale Custom|PlaySoundFireballStart _audiocomponent)))
    (:Is%20Not%20Valid
      _))
  (CallFunction|PlaySound "/Game/SFX/SFX_Fireball_Cue.SFX_Fireball_Cue")
  (CallFunction|PlaySound (select (Math|Random|RandomBoolwithWeight 0.1) "/Game/SFX/SFX_VFX_SpellReady2.SFX_VFX_SpellReady2" "/Game/SFX/SFX_VFX_SpellReady3.SFX_VFX_SpellReady3")))

(event Custom|PlaySoundFireballNotReady
  (bind _asmain_player_bp (Utilities|Casting|CastToMainPlayerBP (Variables|/Script/Engine.Actor|GetInstigator (Components|GetOwner))))
  (Default|PlaySound (Variables|/Game/Blueprints/Characters/MainPlayerBP.MainPlayerBP_C|GetPlayerSoundEffectsManagerCBP _asmain_player_bp) "/Game/SFX/SFX_VFX_SpellFailure2.SFX_VFX_SpellFailure2"))