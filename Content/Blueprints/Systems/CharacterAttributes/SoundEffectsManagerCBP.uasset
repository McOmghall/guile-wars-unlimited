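; Sound effects manager component that plays attached sounds for its owning actor and keeps track of them.
; PlaySound spawns a sound on an optional override component, falling back to itself, passes the owner's location and rotation, and records the returned audio component.
; Spawned sounds stop if their attach target is destroyed.
; DestroyAllSpawnedSounds briefly fades out every valid tracked sound to silence, without clearing the list.
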(event Custom|DestroyAllSpawnedSounds
  (for _array_element (Variables|Default|GetSpawnedSounds)
    (Utilities|IsValid _array_element
      (:Is%20Valid
        (Audio|Components|Audio|FadeOut _array_element 1.0 0.0 :!class /Script/Engine.AudioComponent)))))

(fn PlaySound
  (params (Sound :type Sound%20Base%20Object%20Reference) (OverrideAudioSource :type Scene%20Component%20Object%20Reference))
  (bind _returnvalue (Components|GetOwner))
  (bind _returnvalue_2 (Transformation|GetActorTransform _returnvalue))
  (bind _returnvalue_3 (Audio|SpawnSoundAttached Sound (select (Utilities|IsValid OverrideAudioSource) OverrideAudioSource self) "None" (.location _returnvalue_2) (.rotation _returnvalue_2) "KeepRelativeOffset" true))
  (Utilities|Array|Add (Variables|Default|GetSpawnedSounds) _returnvalue_3)
  (return _returnvalue_3))