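; Actor component that scales its owner's walk speed as a fraction of the speed it had at BeginPlay.
; On BeginPlay it finds the owner's CharacterMovementComponent and caches its MaxWalkSpeed as the initial velocity.
; LerpVelocity sets MaxWalkSpeed between zero and that cached value by an alpha, and Reset calls it at full alpha to restore the original speed.
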(event EventBeginPlay
  (bind _returnvalue (Components|GetOwner))
  (bind _returnvalue_2 (Actor|GetComponentbyClass _returnvalue "/Script/Engine.CharacterMovementComponent"))
  (Utilities|IsValid _returnvalue_2
    (:Is%20Valid
      (bind _output_get (Variables|Default|SetMovementComponent _returnvalue_2))
      (Variables|Default|SetInitialVelocity (Variables|/Script/Engine.CharacterMovementComponent|GetMaxWalkSpeed _output_get)))))

(fn LerpVelocity
  (params (Alpha :type Float%20%28single-precision%29))
  (Variables|/Script/Engine.CharacterMovementComponent|SetMaxWalkSpeed (Variables|Default|GetMovementComponent) (Math|Float|Lerp 0.0 (Variables|Default|GetInitialVelocity) Alpha)))

(fn Reset
  (CallFunction|LerpVelocity 1.0))