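; Sound effects manager component that delegates playback to the player who instigated its owning actor.
; It overrides PlaySound: without a valid override audio source, it casts the owner's Instigator to MainPlayerBP and passes that player's PlayerSoundEffectsManagerCBP to the parent implementation as the source.
; A valid override passes through unchanged.
; If the player or its manager is missing, the parent is not called.
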(event EventBeginPlay
  (|CallParentFunction))

(event EventTick
  (params (DeltaSeconds :type Float%20%28single-precision%29)))

(fn PlaySound
  (params (Sound :type Sound%20Base%20Object%20Reference) (OverrideAudioSource :type Scene%20Component%20Object%20Reference))
  (if (not (Utilities|IsValid OverrideAudioSource))
    (bind _asmain_player_bp (Utilities|Casting|CastToMainPlayerBP (Variables|/Script/Engine.Actor|GetInstigator (Components|GetOwner))))
    (Utilities|IsValid _asmain_player_bp
      (:Is%20Valid
        (Utilities|IsValid (Variables|/Game/Blueprints/Characters/MainPlayerBP.MainPlayerBP_C|GetPlayerSoundEffectsManagerCBP _asmain_player_bp)
          (:Is%20Valid
            (bind _audiocomponent (|CallParentFunction Sound (Variables|/Game/Blueprints/Characters/MainPlayerBP.MainPlayerBP_C|GetPlayerSoundEffectsManagerCBP _asmain_player_bp))) ; Play sound on parent component
            (return _audiocomponent)))))
    (else
      (bind _audiocomponent_2 (|CallParentFunction Sound OverrideAudioSource)) ; Play sound on override component
      (return _audiocomponent_2))))