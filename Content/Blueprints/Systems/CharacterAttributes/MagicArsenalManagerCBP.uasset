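; Player component that manages the magic arsenal: a set of selectable spells plus one separate utility spell.
; On BeginPlay it spawns a SpellManager actor per spell class in the Spells map, passing mana cost and cooldown, and another for the utility spell.
; Next and previous rotate the selected index by modulo and flag the active manager as Selected.
; Start functions delegate casting to the relevant manager and return its fire result and spell.
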(event EventBeginPlay
  (bind _spells (Variables|SpellArsenal|GetSpells))
  (bind _utilityspell (Variables|UtilitySpellArsenal|GetUtilitySpell))
  ;[1 1 1] CREATE MANAGERS FOR ALL SPELLS
  (bind _asmain_player_bp (Utilities|Casting|CastToMainPlayerBP (Components|GetOwner)))
  (bind _keys (Utilities|Map|Keys _spells))
  (for (_array_element _array_index) _keys ; Create all the needed spell managers for our current arsenal
    (bind _returnvalue (Game|SpawnActorfromClass (Variables|SpellArsenal|GetSpellManagerClass) (Transformation|GetActorTransform _asmain_player_bp) "AlwaysSpawn" 0 _array_element (.ManaCost (Utilities|Struct|BreakSpellMetadataStruct (select (.ReturnValue (Utilities|Map|Find _spells _array_element)) (.Value (Utilities|Map|Find _spells _array_element)) (Utilities|Struct|MakeSpellMetadataStruct 0.0 0.0)))) (.Cooldown (Utilities|Struct|BreakSpellMetadataStruct (select (.ReturnValue (Utilities|Map|Find _spells _array_element)) (.Value (Utilities|Map|Find _spells _array_element)) (Utilities|Struct|MakeSpellMetadataStruct 0.0 0.0)))) _asmain_player_bp))
    (Utilities|Map|Add (Variables|SpellArsenal|GetManagedSpells) _array_index _returnvalue))
  (Utilities|FlowControl|Sequence
    (:then_0
      (CallFunction|ChangeActiveSpelltoIndex) ; Select 1st spell as active
    )
    (:then_1
      (bind _returnvalue_2 (Game|SpawnActorfromClass (Variables|SpellArsenal|GetSpellManagerClass) (Transformation|GetActorTransform _asmain_player_bp) "AlwaysSpawn" 0 (.spell _utilityspell) (.manacost (.metadata _utilityspell)) (.cooldown (.metadata _utilityspell)) _asmain_player_bp)) ; Create manager for utility spell
      (Variables|UtilitySpellArsenal|SetUtilitySpellManager _returnvalue_2))))

(fn NextSpell
  (bind (_nextspell _nextspellindex) (CallFunction|RotateSpell 1))
  (return _nextspell _nextspellindex))

(fn RotateSpell
  (params (Rotation :type Integer))
  (bind _keys (Utilities|Map|Keys (Variables|SpellArsenal|GetSpells)))
  (bind _newindex (CallFunction|ChangeActiveSpelltoIndex (Math|Integer|%(Integer) (+ Rotation (Variables|SpellArsenal|GetCurrentSelectedSpell)) (Utilities|Array|Length _keys))))
  (return (Utilities|Array|Get(acopy) _keys _newindex) _newindex))

(fn PrevSpell
  (bind (_nextspell _nextspellindex) (CallFunction|RotateSpell -1))
  (return _nextspell _nextspellindex))

(fn StartCurrentSpell
  (bind _currentselectedspell (Variables|SpellArsenal|GetCurrentSelectedSpell))
  (bind _managedspells (Variables|SpellArsenal|GetManagedSpells))
  (bind (_value _returnvalue) (Utilities|Map|Find _managedspells _currentselectedspell))
  (if _returnvalue
    (bind (_fireresult _spell) (Default|StartSpell _value))
    (return _fireresult _spell)
    (else
      (return "NewEnumerator3" 0))))

(fn ChangeActiveSpelltoIndex
  (params (Index :type Integer))
  (bind _managedspells (Variables|SpellArsenal|GetManagedSpells))
  (Variables|/Game/Blueprints/Systems/CharacterAttributes/SpellManagerBP.SpellManagerBP_C|SetSelected? (.Value (Utilities|Map|Find _managedspells (Variables|SpellArsenal|GetCurrentSelectedSpell))) false)
  (bind _output_get (Variables|SpellArsenal|SetCurrentSelectedSpell Index))
  (Variables|/Game/Blueprints/Systems/CharacterAttributes/SpellManagerBP.SpellManagerBP_C|SetSelected? (.Value (Utilities|Map|Find _managedspells _output_get)) true)
  (return Index))

(fn StartCurrentUtilitySpell
  (bind _utilityspellmanager (Variables|UtilitySpellArsenal|GetUtilitySpellManager))
  (Utilities|IsValid _utilityspellmanager
    (:Is%20Valid
      (bind (_fireresult _spell) (Default|StartSpell _utilityspellmanager))
      (return _fireresult _spell))
    (:Is%20Not%20Valid
      (return "NewEnumerator3" 0))))