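; Player sound effects manager that plays cues for spell casting, mana shield, game start and death.
; Each event plays its own cue, with weighted random picks for some voice variants, including rare Grand Magus easter eggs.
; A failed spell always plays a snap-fail sound, while a gate and reset timer throttle the extra voice line, chosen by failure reason, to once every few seconds.
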(event Custom|PlaySpellStarted
  (CallFunction|PlaySound "/Game/SFX/SFX_Snap1_Cue.SFX_Snap1_Cue"))

(event Custom|PlayAtShieldOn
  (CallFunction|PlaySound "/Game/SFX/SFX_ManaShieldOn.SFX_ManaShieldOn"))

(event Custom|PlayOnDeath
  (CallFunction|PlaySound (select (Math|Random|RandomBoolwithWeight 0.5) "/Game/SFX/SFX_VFX_Death2.SFX_VFX_Death2" "/Game/SFX/SFX_VFX_Death1.SFX_VFX_Death1")))

(event Custom|PlayAtStart
  (CallFunction|PlaySound (select (Math|Random|RandomBoolwithWeight 0.01) "/Game/SFX/SFX_VFX_GrandMagus.SFX_VFX_GrandMagus" "/Game/SFX/SFX_VFX_Begin.SFX_VFX_Begin")))

(event Custom|PlaySpellLaunched
  (CallFunction|PlaySound "/Game/SFX/SFX_Snap2_Cue.SFX_Snap2_Cue"))

(event Custom|ResetSpellFailedSound
  (bind _returnvalue (Math|Random|RandomBoolwithWeight 0.01))
  (bind _returnvalue_2 (select _returnvalue "/Game/SFX/SFX_VFX_GrandMagus.SFX_VFX_GrandMagus" 0))
  (Utilities|FlowControl|Gate false) ; enters at Open
)

(event Custom|PlaySpellFailed
  (params (Reason :type SpellFireResultEnumBP%20Enum))
  (bind _returnvalue (Math|Random|RandomBoolwithWeight 0.01))
  (bind _returnvalue_2 (select _returnvalue "/Game/SFX/SFX_VFX_GrandMagus.SFX_VFX_GrandMagus" 0))
  (CallFunction|PlaySound "/Game/SFX/SFX_SnapFail_Cue.SFX_SnapFail_Cue")
  (Utilities|FlowControl|Sequence
    (:then_0
      (Utilities|FlowControl|Gate false :!label _label
        (:Exit
          (CallFunction|PlaySound (Utilities|Select :Index Reason :NewEnumerator2 0 :NewEnumerator4 _returnvalue_2 :NewEnumerator0 (select (Math|Random|RandomBoolwithWeight 0.3) "/Game/SFX/SFX_VFX_NoManaDUDE.SFX_VFX_NoManaDUDE" "/Game/SFX/SFX_VFX_NoMana.SFX_VFX_NoMana") :NewEnumerator1 (select (Math|Random|RandomBoolwithWeight 0.4) "/Game/SFX/SFX_VFX_NotYetDUDE.SFX_VFX_NotYetDUDE" "/Game/SFX/SFX_VFX_NotYet.SFX_VFX_NotYet") :NewEnumerator3 _returnvalue_2))
          (Utilities|Time|SetTimerbyEvent (delegate Custom|ResetSpellFailedSound) 5.0))))
    (:then_1
      (goto _label Close))))