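; Health component that builds on an inherited Current/Max attribute pool, treating damage as spending from that pool.
; ReceiveDamage predicts the outcome through CanSpend, fires the damage-received dispatcher, then force-spends the damage.
; It fires the die dispatcher when a successful spend leaves health at zero or below, and returns the remaining health.
; On BeginPlay, an owner starting with no health is destroyed with a printed warning.
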(event EventBeginPlay
  (|CallParentFunction)
  (if (<= (Variables|Default|GetCurrent) 0.0)
    (Development|PrintString "WARNING: Created actor with health 0 or less, destroying")
    (Actor|DestroyActor (Components|GetOwner))))

(fn ReceiveDamage
  (params (Damage :type Float%20%28single-precision%29))
  (bind _max (Variables|Default|GetMax))
  (bind (_healthbeforedamage _healthafterdamage _willdie_) (CallFunction|WillDieifDamaged Damage))
  (Default|CallOnDamageReceived Damage _max _healthafterdamage _willdie_)
  (bind (_remainingafterspending _spent) (CallFunction|Spend Damage true))
  (if (and _spent _willdie_)
    (Default|CallOnDie _max _remainingafterspending (and _spent _willdie_)))
  (return _remainingafterspending))

(fn WillDieifDamaged
  (params (Damage :type Float%20%28single-precision%29))
  (bind (_remainingbeforespending _remainingafterspending) (CallFunction|CanSpend Damage))
  (return _remainingbeforespending _remainingafterspending (<= _remainingafterspending 0.0)))