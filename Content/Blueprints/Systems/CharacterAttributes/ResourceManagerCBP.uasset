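; ResourceManagerCBP is a character-attribute Blueprint that tracks a generic resource as a current value against a maximum, refilled on BeginPlay.
; Earn adds the absolute amount and clamps the result between zero and Max.
; CanSpend checks that the remainder stays within that range, and Spend applies the cost only if it passes or Force is set.
; Forced spends are not clamped, so Current can leave the range.
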(event EventBeginPlay
  (CallFunction|Refill))

(event EventTick
  (params (DeltaSeconds :type Float%20%28single-precision%29)))

(fn CanSpend
  (params (Amount :type Float%20%28single-precision%29))
  (bind _current (Variables|Default|GetCurrent))
  (bind _returnvalue (- _current Amount))
  (return _current _returnvalue (and (>= _returnvalue 0.0) (<= _returnvalue (Variables|Default|GetMax)))))

(fn Earn
  (params (Amount :type Float%20%28single-precision%29))
  (bind _output_get (Variables|Default|SetCurrent (Math|Float|Clamp(Float) (+ (Math|Float|Absolute(Float) Amount) (Variables|Default|GetCurrent)) 0.0 (Variables|Default|GetMax))))
  (return _output_get))

(fn Refill
  (bind _output_get (Variables|Default|SetCurrent (Variables|Default|GetMax)))
  (return _output_get))

(fn Spend
  (params (Amount :type Float%20%28single-precision%29) (Force :type Boolean))
  (bind (_remainingbeforespending _remainingafterspending _canspend) (CallFunction|CanSpend Amount))
  (bind _output_get (Variables|Default|SetCurrent (select (or _canspend Force) _remainingafterspending _remainingbeforespending)))
  (return _output_get (or _canspend Force)))