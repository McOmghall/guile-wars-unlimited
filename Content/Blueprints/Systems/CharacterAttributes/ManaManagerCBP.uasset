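; ManaManagerCBP is a character attribute component that manages mana as a spendable, self-recharging resource.
; Each tick it earns mana at ManaRechargePerSecond scaled by delta time, using the inherited Earn function.
; CanSpendMana and SpendMana wrap the parent's generic CanSpend and Spend with mana-named outputs, and spending is never forced.
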(event EventBeginPlay
  (|CallParentFunction))

(event EventTick
  (params (DeltaSeconds :type Float%20%28single-precision%29))
  (|CallParentFunction DeltaSeconds)
  (CallFunction|Earn (* DeltaSeconds (Variables|Default|GetManaRechargePerSecond))) ; Mana recharges over time
)

(fn CanSpendMana
  (params (Amount :type Float%20%28single-precision%29))
  (bind (_remainingbeforespending _remainingafterspending _canspend) (CallFunction|CanSpend Amount))
  (return _remainingbeforespending _remainingafterspending _canspend))

(fn SpendMana
  (params (Amount :type Float%20%28single-precision%29))
  (bind (_remainingafterspending _spent) (CallFunction|Spend Amount false))
  (return _remainingafterspending _spent))