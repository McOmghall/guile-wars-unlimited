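; Base game mode that ends a duel between the player and a single enemy mage when either one dies.
; BeginPlay binds both characters' death events, recording who died first as the win result and unbinding both afterwards.
; At game end it possesses a dummy menu-control character spawned behind and above the player pawn.
; A timeline then drives global time dilation and triggers the win/lose widget, which replaces the main UI.
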(event Custom|EnemyDiedFirst
  (Variables|Default|SetEnemyDiedFirst? true)
  (CallFunction|EndOfGame))

(event Custom|EndOfGame
  (bind _returnvalue (Game|GetPlayerController 0))
  (bind _returnvalue_2 (Game|Player|GetPlayerPawn 0))
  (bind _returnvalue_3 (Transformation|GetActorTransform _returnvalue_2))
  (Utilities|FlowControl|Sequence
    (:then_0
      (EventDispatchers|UnbindallEventsfromOnDieforGameMode (Variables|Default|GetEnemy)) ; Unbind events from the other mage
    )
    (:then_1
      (EventDispatchers|UnbindallEventsfromOnDieforGameMode (Variables|Default|GetPlayer)) ; Unbind event from self
    )
    (:then_2
      (bind _returnvalue_4 (Game|SpawnActorfromClass "/Game/Blueprints/Systems/AuxFunctions/DummyCharacterToControlMenusBP.DummyCharacterToControlMenusBP_C" (Math|Transform|MakeTransform (+ (.location _returnvalue_3) (* (Transformation|GetActorUpVector _returnvalue_2) 1e+02) (* (Transformation|GetActorForwardVector _returnvalue_2) -2e+02)) (.rotation _returnvalue_3) (.scale _returnvalue_3)) "AlwaysSpawn" 0 0))
      (Input|EnableInput _returnvalue_4 _returnvalue)
      (Pawn|Possess _returnvalue _returnvalue_4))
    (:then_3
      (bind _globaltimedilation (Timeline|EndOfGameTimeline Play)
        (:Update
          (Utilities|Time|SetGlobalTimeDilation _globaltimedilation))
        (:SpawnMenu
          (bind _returnvalue_5 (UserInterface|CreateWidget "/Game/Blueprints/UI/UserWidgets/EndOfGameWidgetBP.EndOfGameWidgetBP_C" (Game|GetPlayerController 0) (Variables|Default|GetEnemyDiedFirst?)))
          (UserInterface|Viewport|AddtoPlayerScreen _returnvalue_5 1000)
          (bind _foundwidgets (Widget|GetAllWidgetsOfClass "/Game/Blueprints/UI/UserWidgets/MainUIWidgetBP.MainUIWidgetBP_C" true))
          (for _array_element _foundwidgets
            (Widget|RemovefromParent _array_element)))))))

(event Custom|PlayerDiedFirst
  (Variables|Default|SetEnemyDiedFirst? false)
  (CallFunction|EndOfGame))

(event EventBeginPlay
  (Utilities|FlowControl|Sequence
    (:then_0
      (bind _outactors (Actor|GetAllActorsOfClass "/Game/Blueprints/Characters/EnemyExampleBP.EnemyExampleBP_C"))
      (bind _output_get (Variables|Default|SetEnemy (Utilities|Array|Get(acopy) _outactors)))
      (EventDispatchers|BindEventtoOnDieforGameMode _output_get (delegate Custom|EnemyDiedFirst)))
    (:then_1
      (bind _asmain_player_bp (Utilities|Casting|CastToMainPlayerBP (Game|Player|GetPlayerPawn 0)))
      (bind _output_get_2 (Variables|Default|SetPlayer _asmain_player_bp))
      (EventDispatchers|BindEventtoOnDieforGameMode _output_get_2 (delegate Custom|PlayerDiedFirst)))))

(fn ConstructionScript)