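; Player character that casts spells and switches between free-roam and auto-aim camera modes.
; Auto-aim smoothly turns the camera toward the nearest TargetableBPInterface actor, falling back to free roam, where spells target a forward point.
; Pressing cast readies a spell and release shoots it, with timelines driving camera follow rate, crosshair focus, animation blends and movement slowdown.
; Manager components handle spells, mana, health and speed, with debug refill keys.
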(event Custom|StartFocus
  ;[0.6422 0.08257 0.01835 0.367] Spell Management
  ;;[0.1009 0.2936 0.1009] Animation For Intensity and Focus Effect (on Shoots)
  (bind (_direction _focuspercentageforwards _focuspercentagebackwards) (Timeline|FocusAnimation Play)
    (:Update
      (Utilities|FlowControl|Sequence
        (:then_0
          (Variables|Control|SetCameraRotationRate (Utilities|Select :Index _direction :Forward _focuspercentageforwards :Backward _focuspercentagebackwards)))
        (:then_1
          (bind _asbase_magic_crosshair_bp (Utilities|Casting|CastToBaseMagicCrosshairBP (Variables|/Script/Engine.ChildActorComponent|GetChildActor (Variables|Default|GetRealCrosshair))))
          (Variables|/Game/Blueprints/UI/DiegeticElements/BaseMagicCrosshairBP.BaseMagicCrosshairBP_C|SetFocusAlpha _asbase_magic_crosshair_bp (* (Utilities|Select :Index _direction :Forward _focuspercentageforwards :Backward _focuspercentagebackwards) (Utilities|Select :Index (Variables|Control|GetControlMode) :NewEnumerator3 1.0 :NewEnumerator2 1.0 :NewEnumerator1 2.0))))))))

(event Custom|ReverseFocus
  ;[0.6422 0.08257 0.01835 0.367] Spell Management
  ;;[0.1009 0.2936 0.1009] Animation For Intensity and Focus Effect (on Shoots)
  (bind (_direction _focuspercentageforwards _focuspercentagebackwards) (Timeline|FocusAnimation Reverse)
    (:Update
      (Utilities|FlowControl|Sequence
        (:then_0
          (Variables|Control|SetCameraRotationRate (Utilities|Select :Index _direction :Forward _focuspercentageforwards :Backward _focuspercentagebackwards)))
        (:then_1
          (bind _asbase_magic_crosshair_bp (Utilities|Casting|CastToBaseMagicCrosshairBP (Variables|/Script/Engine.ChildActorComponent|GetChildActor (Variables|Default|GetRealCrosshair))))
          (Variables|/Game/Blueprints/UI/DiegeticElements/BaseMagicCrosshairBP.BaseMagicCrosshairBP_C|SetFocusAlpha _asbase_magic_crosshair_bp (* (Utilities|Select :Index _direction :Forward _focuspercentageforwards :Backward _focuspercentagebackwards) (Utilities|Select :Index (Variables|Control|GetControlMode) :NewEnumerator3 1.0 :NewEnumerator2 1.0 :NewEnumerator1 2.0))))))))

(event Custom|ConsumeMana
  (params (Amount :type Float%20%28single-precision%29))
  ;[0.6422 0.08257 0.01835 0.367] Spell Management
  ;;[0.1009 0.2936 0.1009] Mana Consumption
  (Default|SpendMana (Variables|Default|GetManaManagerCBP) Amount))

(event Custom|SpellReady
  ;[0.6422 0.08257 0.01835 0.367] Spell Management
  ;;[0.1009 0.2936 0.1009] Spell is Ready
  (Audio|Components|Audio|Stop (Variables|Default|GetReadySpellAnimations))
  (Default|Reset (Variables|Default|GetSpeedModifiersManagerCBP)))

(event EventTick
  (params (DeltaSeconds :type Float%20%28single-precision%29))
  (bind _returnvalue (Input|AxisValues|GetTurnRate))
  (bind _returnvalue_2 (Input|AxisValues|GetLookUpRate))
  ;[0.2385 0.422 1 0.367] Camera Handling (Camera Modes)
  (switch Utilities|FlowControl|Switch|SwitchonControlModeEnumBP (Variables|Control|GetControlMode) ; AUTO AIM: Takes an objective and makes the camera follow it\nFREE ROAM: Player can control the camera with the TurnRate/LookUpRate axis (rigth joystick)\nFREE ROAM INIT: Happens before being in Free Roam state (can be used to orient the camera before handling control back to the player)
    (:NewEnumerator3
      (if (> (+ (Math|Float|Absolute(Float) _returnvalue) (Math|Float|Absolute(Float) _returnvalue_2)) 0.0) ; When the player moves the camera joystick\ncontrol is handled back immediately
        (Variables|Control|SetControlMode "NewEnumerator2")
        (Class|MyProjectCharacter|TurnatRate _returnvalue :!label _label)
        (Class|MyProjectCharacter|LookUpatRate _returnvalue_2)))
    (:NewEnumerator2
      (goto _label))
    (:NewEnumerator1
      (Utilities|IsValid (Utilities|ToObject(Interface) (Variables|Control|GetCurrentTarget))
        (:Is%20Valid
          (bind _location (Default|GetTargetableLocation (Variables|Control|GetCurrentTarget) :!label _label_2))
          (Pawn|SetControlRotation (Pawn|GetController) (CallFunction|RotationCameratoTargetSmooth _location (Variables|Control|GetCameraRotationRate))))
        (:Is%20Not%20Valid
          (bind (_target _newcontrolmode _ok _istargetingmode) (CallFunction|GetNewTargetbyControlMode (Variables|Control|GetControlMode)))
          (if (and _ok _istargetingmode)
            (goto _label_2)
            (else
              (Development|PrintString "Not found objective?  
Safely return to Free Roam Mode")
              (bind _output_get (Variables|Control|SetControlMode "NewEnumerator2"))
              (CallFunction|GetNewTargetbyControlMode _output_get))))))))

(event EventBeginPlay
  ;[0.2385 0.422 1 0.367] Camera Handling (Camera Modes)
  ;;[0.1009 0.2936 0.01835] Input Action AutoAimToggle (Switch between control modes)
  (CallFunction|GetNewTargetbyControlMode (Utilities|Select :Index (Variables|Control|GetControlMode) :NewEnumerator3 "NewEnumerator1" :NewEnumerator2 "NewEnumerator1" :NewEnumerator1 "NewEnumerator3")))

(event Input|ActionEvents|InputActionAutoAimToggle
  (params (Key :type Key%20Structure :default "AnyKey"))
  ;[0.2385 0.422 1 0.367] Camera Handling (Camera Modes)
  ;;[0.1009 0.2936 0.01835] Input Action AutoAimToggle (Switch between control modes)
  (:Pressed
    (CallFunction|GetNewTargetbyControlMode (Utilities|Select :Index (Variables|Control|GetControlMode) :NewEnumerator3 "NewEnumerator1" :NewEnumerator2 "NewEnumerator1" :NewEnumerator1 "NewEnumerator3"))))

(event Input|ActionEvents|InputActionCastCurrentSpell
  (params (Key :type Key%20Structure :default "AnyKey"))
  (bind _returnvalue (Input|AxisValues|GetMoveRight))
  (bind _controlmode (Variables|Control|GetControlMode))
  (bind _returnvalue_2 (* _returnvalue 1e+02))
  ;[0.6422 0.08257 0.01835 0.367] Spell Management
  (:Pressed
    (bind (_fireresult _spellresult) (Default|StartCurrentSpell (Variables|Default|GetMagicArsenalManagerCBP)))
    (switch Utilities|FlowControl|Switch|SwitchonSpellFireResultEnumBP _fireresult
      (:NewEnumerator2
        (CallFunction|StartFocus)
        (Components|Timeline|PlayfromStart (Variables|Default|GetReadySpellAnimations)))))
  (:Released
    (switch Utilities|FlowControl|Switch|SwitchonSpellFireResultEnumBP _fireresult
      (:NewEnumerator2
        (Utilities|IsValid _spellresult
          (:Is%20Valid
            (CallFunction|ReverseFocus)
            (Components|Timeline|PlayfromStart (Variables|Default|GetLaunchSpellAnimations))
            (Default|Shoot _spellresult (Variables|Control|GetCurrentTarget) (Math|Vector|MakeVector 3e+03 (Utilities|Select :Index _controlmode :NewEnumerator3 _returnvalue_2 :NewEnumerator2 _returnvalue_2 :NewEnumerator1 (* _returnvalue 1e+02)) (Utilities|Select :Index _controlmode :NewEnumerator3 1e+02 :NewEnumerator2 1e+02 :NewEnumerator1 1e+02))))
          (:Is%20Not%20Valid
            _)))
      (:NewEnumerator4
        _)
      (:NewEnumerator3
        _))
    ;;[0.1009 0.2936 0.1009] Spell is Ready
    (Audio|Components|Audio|Stop (Variables|Default|GetReadySpellAnimations))
    (Default|Reset (Variables|Default|GetSpeedModifiersManagerCBP))))

(event Input|KeyboardEvents|M
  (params (Key :type Key%20Structure :default "AnyKey"))
  (:Pressed
    (Default|Refill (Variables|Default|GetManaManagerCBP))))

(event Input|KeyboardEvents|H
  (params (Key :type Key%20Structure :default "AnyKey"))
  (:Pressed
    (Default|Refill (Variables|Default|GetHealthManagerCBP))))

(fn ConstructionScript)

(fn RotationCameratoTarget
  (params (Target :type Vector%20%28by%20ref%29))
  (return (Math|Rotator|FindLookatRotation (Transformation|GetWorldLocation (Variables|Default|GetFollowCamera)) Target)))

(fn RotationCameratoTargetSmooth
  (params (Target :type Vector) (Alpha :type Float%20%28single-precision%29))
  (return (Math|Rotator|Lerp(Rotator) (Pawn|GetControlRotation :!class /Script/Engine.Pawn) (CallFunction|RotationCameratoTarget Target) Alpha true)))

(fn UpdateTargetandControlMode
  (params (Target :type Targetable%20BP%20Interface%20Interface) (ControlMode :type ControlModeEnumBP%20Enum))
  (Variables|Control|SetControlMode ControlMode)
  (bind _output_get (Variables|Control|SetCurrentTarget Target))
  (bind _asbase_magic_crosshair_bp (Utilities|Casting|CastToBaseMagicCrosshairBP (Variables|/Script/Engine.ChildActorComponent|GetChildActor (Variables|Default|GetRealCrosshair)))
    (:then
      (Default|ControlModeChange _asbase_magic_crosshair_bp ControlMode _output_get))
    (:CastFailed
      _))
  (return _output_get ControlMode))

(fn FindBestTarget
  (params (TargetArray :type Array%20of%20Actor%20Object%20References) (RemoveSelfTargets :type Actor%20Object%20Reference%20%28by%20ref%29))
  (Utilities|Array|RemoveItem TargetArray RemoveSelfTargets)
  (if (> (Utilities|Array|Length TargetArray) 0)
    (for (_array_element _array_index) TargetArray
      ;[1 1 1] Find Nearest Target
      (Utilities|IsValid _array_element
        (:Is%20Valid
          (LocalVariables|SetIndexOfNearestEnemy (select (< (Math|Vector|VectorLengthSquared (- (Transformation|GetActorLocation) (Transformation|GetActorLocation _array_element))) (LocalVariables|GetCurrentMaxDistanceToObjective)) _array_index (LocalVariables|GetIndexOfNearestEnemy)))
          (LocalVariables|SetCurrentMaxDistanceToObjective (select (< (Math|Vector|VectorLengthSquared (- (Transformation|GetActorLocation) (Transformation|GetActorLocation _array_element))) (LocalVariables|GetCurrentMaxDistanceToObjective)) (Math|Vector|VectorLengthSquared (- (Transformation|GetActorLocation) (Transformation|GetActorLocation _array_element))) (LocalVariables|GetCurrentMaxDistanceToObjective)))))))
  ;[1 1 1] Return Result of Search
  (return (.HasResult? (Utilities|FindwithBoundsCheck TargetArray (LocalVariables|GetIndexOfNearestEnemy))) (.Result (Utilities|FindwithBoundsCheck TargetArray (LocalVariables|GetIndexOfNearestEnemy)))))

(fn CanSpendMana
  (params (Amount :type Float%20%28single-precision%29))
  (bind (_remainingbeforespendingmana _remainingafterspendingmana _canspendmana) (Default|CanSpendMana (Variables|Default|GetManaManagerCBP) Amount))
  (return _remainingbeforespendingmana _remainingafterspendingmana _canspendmana))

(fn GetCurrentTarget
  (return (Variables|Control|GetCurrentTarget)))

(fn GetNewTargetbyControlMode
  (params (ControlMode :type ControlModeEnumBP%20Enum))
  (switch Utilities|FlowControl|Switch|SwitchonControlModeEnumBP ControlMode
    (:NewEnumerator3
      _)
    (:NewEnumerator2
      _)
    (:NewEnumerator1
      ;[1 1 1] For Aiming Mode: Find Nearest Targetable and return it
      (bind _outactors (Actor|GetAllActorswithInterface "/Game/Blueprints/Systems/Interfaces/TargetableBPInterface.TargetableBPInterface_C"))
      (bind (_found_ _target) (CallFunction|FindBestTarget _outactors (Variables|/Script/Engine.ChildActorComponent|GetChildActor (Variables|Default|GetShootForwardPoint))))
      (if _found_
        ;;[1 1 1] Return if Found
        (bind _entity (Class|TargetableBPInterface|GetasTarget(Message) _target))
        (bind (_sametarget _samecontrolmode) (CallFunction|UpdateTargetandControlMode _entity ControlMode))
        (return _sametarget _samecontrolmode true true)
        (else
          ;;[1 1 1] Safely Go Back to NON TARGETING control mode if there are no targetable objects
          (bind (_target_2 _newcontrolmode _ok _istargetingmode) (CallFunction|GetNewTargetbyControlMode "NewEnumerator2"))
          (return _target_2 _newcontrolmode _ok _istargetingmode)))))
  ;[1 1 1] FreeRoam Modes just shoot ahead
  (bind _entity_2 (Class|TargetableBPInterface|GetasTarget(Message) (Variables|/Script/Engine.ChildActorComponent|GetChildActor (Variables|Default|GetShootForwardPoint))))
  (bind (_sametarget_2 _samecontrolmode_2) (CallFunction|UpdateTargetandControlMode _entity_2 ControlMode))
  (return _sametarget_2 _samecontrolmode_2 true false))

(fn ReceiveDamage
  (params (Damage :type Float%20%28single-precision%29))
  (bind _remainingdamage (Default|ReceiveDamage (Variables|Default|GetHealthManagerCBP) Damage))
  (return _remainingdamage))

(fn SpendMana
  (params (Amount :type Float%20%28single-precision%29))
  (bind (_remainingafterspendingmana _spent) (Default|SpendMana (Variables|Default|GetManaManagerCBP) Amount))
  (return _remainingafterspendingmana _spent))

(fn WillDieifDamaged
  (params (Damage :type Float%20%28single-precision%29))
  (return 0.0 0.0 false))