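; Base actor for a diegetic magic crosshair, built from two planes that spin continuously.
; Each tick it blends between minimum and maximum rotation speeds by an acceleration alpha and scales the result by delta time.
; The first plane turns by that amount, while the second counter-rotates at half the rate.
; The alpha is only read here, never set.
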(event EventBeginPlay)

(event Collision|EventActorBeginOverlap
  (params (OtherActor :type Actor%20Object%20Reference)))

(event EventTick
  (params (DeltaSeconds :type Float%20%28single-precision%29))
  (bind _rootrotationspeedmin (Variables|CrosshairConfig|GetRootRotationSpeedMin))
  (bind _rootrotationspeedmax (Variables|CrosshairConfig|GetRootRotationSpeedMax))
  (bind _accelerationalpha (Variables|CrosshairConfig|GetAccelerationAlpha))
  (bind _returnvalue (Math|Rotator|Lerp(Rotator) _rootrotationspeedmin _rootrotationspeedmax _accelerationalpha true))
  (bind _returnvalue_2 (* _returnvalue DeltaSeconds))
  (Transformation|AddRelativeRotation (Variables|Default|GetPlane0) _returnvalue_2 false false)
  (Transformation|AddRelativeRotation (Variables|Default|GetPlane1) (* (Class|KismetMathLibrary|NegateRotator _returnvalue_2) 0.5) false false))

(fn ConstructionScript)