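; FollowerCBP computes a launch transform positioned relative to RelativeActor and aimed at CurrentTarget.
; GetRelativePositionToActor rotates StartingOffset by that actor's rotation, adds its location, and faces the target's targetable location at unit scale.
; Tick calls this function every frame but leaves the result unused and only prints "Fire", so nothing is moved or launched here.
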(event EventBeginPlay)

(event EventTick
  (params (DeltaSeconds :type Float%20%28single-precision%29))
  (CallFunction|GetRelativePositiontoActor)
  (Development|PrintString "Fire"))

(fn GetRelativePositiontoActor
  (bind _relativeactor (Variables|Default|GetRelativeActor))
  (bind _startingoffset (Variables|Default|GetStartingOffset))
  (bind _returnvalue (Transformation|GetActorTransform _relativeactor))
  (bind _returnvalue_2 (Math|Vector|RotateVector _startingoffset (.rotation _returnvalue)))
  (bind _returnvalue_3 (+ (.location _returnvalue) _returnvalue_2))
  (bind _location (Default|GetTargetableLocation (Variables|Default|GetCurrentTarget)))
  (return (Math|Transform|MakeTransform _returnvalue_3 (Math|Rotator|FindLookatRotation _returnvalue_3 _location) "1.000000,1,1")))