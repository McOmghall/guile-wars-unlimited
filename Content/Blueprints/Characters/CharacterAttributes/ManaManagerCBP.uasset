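; Mana manager component Blueprint for characters that holds a mana pool and answers spending requests.
; CurrentMana fills to MaxMana on BeginPlay, and CanSpendMana reports the current value and whether it covers a requested amount.
; SpendMana builds on that check to return a success flag and the resulting remainder, but never writes that remainder back to CurrentMana.
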(event EventBeginPlay
  (Variables|Default|SetCurrentMana (Variables|Default|GetMaxMana)))

(fn CanSpendMana
  (params (Amount :type Float%20%28single-precision%29))
  (bind _currentmana (Variables|Default|GetCurrentMana))
  (return _currentmana (>= _currentmana Amount)))

(fn SpendMana
  (params (Amount :type Float%20%28single-precision%29))
  (bind (_remainingbeforespendingmana _canspendmana) (CallFunction|CanSpendMana Amount))
  (return (select _canspendmana (- _remainingbeforespendingmana Amount) _remainingbeforespendingmana) _canspendmana))