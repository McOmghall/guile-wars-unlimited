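; Player component that manages the magic arsenal, handling spell selection and casting for MainPlayerBP.
; On BeginPlay it spawns one spell manager actor per Spells entry at the player and maps it by array index.
; NextSpell and PrevSpell step the selected index through RotateSpell, which applies a modulo by the array length.
; StartCurrentSpell forwards to the selected manager's StartSpell, returning its fire result and spell, or a fallback result if none exists.
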(event EventBeginPlay
  (bind _asmain_player_bp (Utilities|Casting|CastToMainPlayerBP (Components|GetOwner)))
  (for (_array_element _array_index) (Variables|Default|GetSpells) ; Create all the needed spell managers for our current arsenal
    (bind _returnvalue (Game|SpawnActorfromClass (Variables|Default|GetSpellManagerClass) (Transformation|GetActorTransform _asmain_player_bp) "AlwaysSpawn" 0 _array_element _asmain_player_bp))
    (Utilities|Map|Add (Variables|Default|GetManagedSpells) _array_index _returnvalue)))

(fn NextSpell
  (bind _nextspellindex (CallFunction|RotateSpell 1))
  (return 0 _nextspellindex))

(fn RotateSpell
  (params (Rotation :type Integer))
  (bind _spells (Variables|Default|GetSpells))
  (bind _output_get (Variables|Default|SetCurrentSelectedSpell (Math|Integer|%(Integer) (+ Rotation (Variables|Default|GetCurrentSelectedSpell)) (Utilities|Array|Length _spells))))
  (return (Utilities|Array|Get(acopy) _spells _output_get) _output_get))

(fn PrevSpell
  (bind _nextspellindex (CallFunction|RotateSpell -1))
  (return 0 _nextspellindex))

(fn StartCurrentSpell
  (bind _currentselectedspell (Variables|Default|GetCurrentSelectedSpell))
  (bind _managedspells (Variables|Default|GetManagedSpells))
  (bind (_value _returnvalue) (Utilities|Map|Find _managedspells _currentselectedspell))
  (if _returnvalue
    (bind (_fireresult _spell) (Default|StartSpell _value))
    (return _fireresult _spell)
    (else
      (return "NewEnumerator3" 0))))