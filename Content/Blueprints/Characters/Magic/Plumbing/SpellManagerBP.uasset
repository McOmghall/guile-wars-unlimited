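; Spell manager actor that spawns a magic spell of its managed class on behalf of its instigator.
; BeginPlay prints an error if the owner is invalid or does not implement the CanAcquireTargets interface.
; StartSpell always spawns the spell at the instigator's transform, passes the instigator along, and returns the spawned spell with a fire result based on its validity.
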(event EventBeginPlay
  (bind _returnvalue (Components|GetOwner))
  (if (not (and (Utilities|IsValid _returnvalue) (Utilities|DoesObjectImplementInterface _returnvalue "/Game/Blueprints/Systems/Interfaces/CanAcquireTargetsBPInterface.CanAcquireTargetsBPInterface_C")))
    (Development|PrintString "ERROR: Not suported instigator, needs to implement CanAcquireTargets interface")))

(fn ConstructionScript)

(fn StartSpell
  (bind _returnvalue (Game|GetInstigator))
  (bind _returnvalue_2 (Game|SpawnActorfromClass (Variables|Default|GetManagedSpellClass) (Transformation|GetActorTransform _returnvalue) "AlwaysSpawn" 0 _returnvalue))
  (return (select (Utilities|IsValid _returnvalue_2) "NewEnumerator2" "NewEnumerator3") _returnvalue_2))