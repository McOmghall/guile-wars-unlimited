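; FollowerCBP is a component that keeps a spell actor at an offset from its Instigator.
; The target transform adds Offset, rotated by the Instigator's rotation, to its location and copies its rotation and scale.
; BeginPlay snaps the owner there; Tick, while ApplyOffset is set, lerps toward it by DeltaSeconds times ApproximationPerSecond.
; Owners that are not SpellBP or lack a valid Instigator keep their current transform.
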(event EventTick
  (params (DeltaSeconds :type Float%20%28single-precision%29))
  (if (Variables|Default|GetApplyOffset)
    (bind _transformtolaunch (CallFunction|GetRelativePositiontoActor))
    (Transformation|SetActorTransform (Components|GetOwner) (Math|Transform|Lerp(Transform) (Transformation|GetActorTransform (Components|GetOwner)) _transformtolaunch (* DeltaSeconds (Variables|Default|GetApproximationPerSecond))))))

(event EventBeginPlay
  (bind _transformtolaunch (CallFunction|GetRelativePositiontoActor))
  (Transformation|SetActorTransform (Components|GetOwner) _transformtolaunch))

(fn GetRelativePositiontoActor
  (bind _asspell_bp (Utilities|Casting|CastToSpellBP (Components|GetOwner))
    (:then
      (Utilities|IsValid (Variables|/Script/Engine.Actor|GetInstigator _asspell_bp)
        (:Is%20Valid
          (return (Math|Transform|MakeTransform (+ (.location (Transformation|GetActorTransform (Variables|/Script/Engine.Actor|GetInstigator _asspell_bp))) (Math|Vector|RotateVector (Variables|Default|GetOffset) (.rotation (Transformation|GetActorTransform (Variables|/Script/Engine.Actor|GetInstigator _asspell_bp))))) (.rotation (Transformation|GetActorTransform (Variables|/Script/Engine.Actor|GetInstigator _asspell_bp))) (.scale (Transformation|GetActorTransform (Variables|/Script/Engine.Actor|GetInstigator _asspell_bp))))))
        (:Is%20Not%20Valid
          _)))
    (:CastFailed
      _))
  (return (Transformation|GetActorTransform (Components|GetOwner))))