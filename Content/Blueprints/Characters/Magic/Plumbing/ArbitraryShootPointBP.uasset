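; ArbitraryShootPointBP is a placeable point in the magic plumbing that can stand in as a target for shots.
; It returns itself as both actor and target, and reports its actor location as the targetable location.
; For homing, it supplies its default scene root with zero gravity scale.
; It holds no active event or construction logic.
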(event EventBeginPlay)

(event Collision|EventActorBeginOverlap
  (params (OtherActor :type Actor%20Object%20Reference)))

(event EventTick
  (params (DeltaSeconds :type Float%20%28single-precision%29)))

(fn ConstructionScript)

(fn GetasActor
  (return self))

(fn GetasTarget
  (return self))

(fn GetHomingComponent
  (return (Variables|Default|GetDefaultSceneRoot) 0.0))

(fn GetTargetableLocation
  (return (Transformation|GetActorLocation)))