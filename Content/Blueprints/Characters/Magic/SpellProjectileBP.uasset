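; Spell projectile that follows its shooter until fired, then homes in on its target and damages what it hits.
; Shoot destroys the follower component, then SetTarget aims along the look-at axes, scaled per axis by ScaleVelocity to allow deviation, and activates movement.
; The target supplies the homing component and acceleration, which the projectile multiplies by its own factor.
; Overlapping an actor implementing DamageableBPInterface sends it Damage and destroys the projectile.
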(event OnComponentBeginOverlap(ProjectileMesh)
  (params (OverlappedComponent :type Primitive%20Component%20Object%20Reference) (OtherActor :type Actor%20Object%20Reference) (OtherComp :type Primitive%20Component%20Object%20Reference) (OtherBodyIndex :type Integer) (bFromSweep :type Boolean) (SweepResult :type Hit%20Result%20Structure%20%28by%20ref%29))
  (if (Utilities|DoesObjectImplementInterface OtherActor "/Game/Blueprints/Systems/Interfaces/DamageableBPInterface.DamageableBPInterface_C") ; Can we damage it?
    (Class|DamageableBPInterface|ReceiveDamage(Message) OtherActor (Variables|Default|GetDamage)) ; If so, damage it.
    (Actor|DestroyActor)))

(event EventAfterShooting
  (|CallParentFunction))

(event EventShoot
  (params (ScaleVelocity :type Vector))
  (|CallParentFunction ScaleVelocity)
  (CallFunction|DeactivateFollower) ; Stop Following movement of shooter
  (bind _modifiedmovementcomponent (CallFunction|SetTarget (Variables|Default|GetProjectileMovement) (Variables|Default|GetTarget) ScaleVelocity)) ; Take Aim
  (Components|Activation|Activate _modifiedmovementcomponent true) ; Fire!
)

(event EventBeforeShooting
  (|CallParentFunction))

(fn ConstructionScript)

(fn DeactivateFollower
  (bind _followercbp (Variables|Default|GetFollowerCBP))
  (Variables|/Game/Blueprints/Characters/Magic/Plumbing/FollowerCBP.FollowerCBP_C|SetApplyOffset _followercbp false)
  (Components|Activation|Deactivate _followercbp)
  (Components|DestroyComponent _followercbp))

(fn SetTarget
  (params (ProjectileMovementComponent :type Projectile%20Movement%20Component%20Object%20Reference) (Target :type Targetable%20BP%20Interface%20Interface) (VelocityScale :type Vector))
  (bind (_x _y _z) (Math|Vector|BreakVector VelocityScale))
  (Utilities|IsValid (Utilities|ToObject(Interface) Target)
    (:Is%20Valid
      (bind _location (Default|GetTargetableLocation Target))
      (Variables|/Script/Engine.MovementComponent|SetVelocity ProjectileMovementComponent (+ (* (Math|Vector|Normalize (Math|Vector|GetForwardVector (Math|Rotator|FindLookatRotation (Transformation|GetActorLocation) _location))) _x) (* (Math|Vector|Normalize (Math|Vector|GetRightVector (Math|Rotator|FindLookatRotation (Transformation|GetActorLocation) _location))) _y) (* (Math|Vector|Normalize (Math|Vector|GetUpVector (Math|Rotator|FindLookatRotation (Transformation|GetActorLocation) _location))) _z))) ; Set velocity of projectile
      (bind (_hometo _homingaccelmag) (Default|GetHomingComponent Target))
      (Variables|/Script/Engine.ProjectileMovementComponent|SetHomingTargetComponent ProjectileMovementComponent _hometo) ; Home In objective by a factor\ngiven by both objective and projectile
      (Variables|/Script/Engine.ProjectileMovementComponent|SetHomingAccelerationMagnitude ProjectileMovementComponent (* _homingaccelmag (Variables|Default|GetHomingAccelMagMultiplier))))
    (:Is%20Not%20Valid
      _))
  (return ProjectileMovementComponent))

(fn DrawDebugTrajectory
  (bind _returnvalue (Transformation|GetActorLocation))
  (Rendering|Debug|DrawDebugLine _returnvalue (+ _returnvalue (* (Transformation|GetVelocity) -1)) (Math|Conversions|ToLinearColor(Vector) (Math|Random|RandomUnitVector)) 1.0 1.0))

(fn DrawDebugDivergence
  (params (Origin :type Vector) (Movement1 :type Vector) (Movement2 :type Vector))
  (Rendering|Debug|DrawDebugLine Origin (+ Origin Movement1) "(R=1.000000,G=0.000000,B=0.000000,A=1.000000)" 1.0 2.0)
  (Rendering|Debug|DrawDebugLine Origin (+ Origin Movement2) "(R=0.000000,G=0.000000,B=1.000000,A=1.000000)" 1.0 2.0))