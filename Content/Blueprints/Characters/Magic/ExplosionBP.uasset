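; ExplosionBP is a magic explosion that registers actors overlapping it during a brief window.
; Each new actor passes through ApplyEffects, a stub here that returns its input, and is stored in AffectedTargets to prevent repeat hits.
; The first overlap starts a one-time 0.2-second delay that destroys the Sphere component.
; The particle system controls lifetime, destroying the actor when it finishes.
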(event OnSystemFinished(ParticleSystem)
  (params (PSystem :type Particle%20System%20Component%20Object%20Reference))
  (Actor|DestroyActor))

(event Collision|EventActorBeginOverlap
  (params (OtherActor :type Actor%20Object%20Reference))
  (bind _affectedtargets (Variables|Default|GetAffectedTargets))
  (Utilities|FlowControl|Sequence
    (:then_0
      (if (< (Utilities|Array|FindItem _affectedtargets OtherActor) 0) ; If we haven't applied effects to this actor\napply them and add it to the array
        (bind _result (CallFunction|ApplyEffects OtherActor))
        (Utilities|Array|Add _affectedtargets _result)))
    (:then_1
      (Utilities|FlowControl|DoOnce false ; Remain in place and get objectives for 0.2 secs
        (:Completed
          (Utilities|FlowControl|Delay 0.2)
          (Components|DestroyComponent (Variables|Default|GetSphere)))))))

(fn ConstructionScript)

(fn ApplyEffects
  (params (To :type Actor%20Object%20Reference))
  (return To))