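; Base magic crosshair actor, a diegetic aiming element that spins and follows an optional target.
; ControlModeChange stores the target and runs a timeline that sets ConvergenceRate for free-roam or auto-aim, logging an error for auto-aim without a target.
; Each tick, FocusAlpha drives spin speed and scale, while ConvergenceRate eases rotation toward the target and slides the crosshair forward by a proportion of target distance, re-centering when none exists.
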(event Custom|ControlModeChange
  (params (To :type ControlModeEnumBP%20Enum) (Target :type Targetable%20Entity%20BP%20Interface%20Interface))
  (bind _returnvalue (Utilities|String|MakeLiteralString "ERROR: Changing to AutoAim without a Target is not allowed"))
  ;[0.3486 0.7431 1 0.7615] ControlModeChange
  (Variables|CrosshairEffectsConfig|SetTarget Target)
  (if (not (and (Utilities|Enum|Equal(Enum) To "NewEnumerator1") (not (Utilities|IsValid (Utilities|ToObject(Interface) Target)))))
    (bind (_direction _freeroamrotationrate _autoaimrotationrate) (Timeline|Timeline_0 PlayFromStart)
      (:Update
        (Variables|CrosshairEffectsConfig|SetConvergenceRate (Utilities|Select :Index To :NewEnumerator2 _freeroamrotationrate :NewEnumerator1 _autoaimrotationrate))))
    (else
      (Development|PrintString _returnvalue true true "(R=1.000000,G=0.073746,B=0.000000,A=1.000000)")
      (Class|VisualLoggerKismetLibrary|LogText _returnvalue "Error"))))

(event EventBeginPlay
  ;[0 0 0 0.3395] Begin Play
  (Variables|CrosshairEffectsConfig|SetBaseCrosshairOffset (Variables|/Script/Engine.SceneComponent|GetRelativeLocation (Variables|Default|GetCrosshairBetweenObjectiveOffset))))

(event EventTick
  (params (DeltaSeconds :type Float%20%28single-precision%29))
  (bind _returnvalue (Transformation|GetActorTransform))
  (bind _returnvalue_2 (Transformation|GetActorTransform))
  (bind _target (Variables|CrosshairEffectsConfig|GetTarget))
  (bind _target_2 (Variables|CrosshairEffectsConfig|GetTarget))
  (bind _focusalpha (Variables|CrosshairEffectsConfig|GetFocusAlpha))
  (bind _returnvalue_3 (Utilities|ToObject(Interface) _target))
  ;[0 0 0 0.3395] Tick
  (Utilities|FlowControl|Sequence
    (:then_0
      ;;[0.1468 0.3028 0.1835 0.844] Focus Effect Management
      (Transformation|AddRelativeRotation (Variables|Default|GetCrosshairSpinAxis) (* (Math|Rotator|Lerp(Rotator) (Variables|CrosshairEffectsConfig|GetRotationSpeedAtMinFocus) (Variables|CrosshairEffectsConfig|GetRotationSpeedAtMaxFocus) (Variables|CrosshairEffectsConfig|GetFocusAlpha) true) DeltaSeconds) false false) ; Rotate by Speed * Time
      (Transformation|SetRelativeScale3D (Variables|Default|GetCrosshairSpinAxis) (Math|Vector|Lerp(Vector) (Variables|/Script/Engine.SceneComponent|GetRelativeScale3D (Variables|Default|GetCrosshairSpinAxis)) (Math|Vector|Lerp(Vector) (Variables|CrosshairEffectsConfig|GetScaleAtMinFocus) (Variables|CrosshairEffectsConfig|GetScaleAtMaxFocus) _focusalpha) (/ (+ (Variables|CrosshairEffectsConfig|GetConvergenceRate) _focusalpha) 2.0))))
    (:then_1
      ;;[0.3761 0.04587 -0.01835 0.789] Rotation to Objective Management
      (Utilities|IsValid (Utilities|ToObject(Interface) _target_2)
        (:Is%20Valid
          (bind _location (Default|GetTargetableLocation _target_2))
          (Transformation|SetRelativeRotation (Variables|Default|GetRootOfCrosshairs) (Math|Rotator|Lerp(Rotator) (Variables|/Script/Engine.SceneComponent|GetRelativeRotation (Variables|Default|GetRootOfCrosshairs)) (Math|Rotator|FindLookatRotation (Math|Vector|MakeVector 0.0 0.0 0.0) (Math|Transform|InverseTransformLocation (Math|Transform|MakeTransform (.location _returnvalue) (.rotation _returnvalue) (.scale _returnvalue)) _location)) (Variables|CrosshairEffectsConfig|GetConvergenceRate) true) false false) ; If we DO have a target, rotate the crosshair towards it
        )
        (:Is%20Not%20Valid
          (Transformation|SetRelativeRotation (Variables|Default|GetRootOfCrosshairs) (Math|Rotator|Lerp(Rotator) (Variables|/Script/Engine.SceneComponent|GetRelativeRotation (Variables|Default|GetRootOfCrosshairs)) "0, 0, 0" (Variables|CrosshairEffectsConfig|GetConvergenceRate) true) false false) ; If we DON'T have a target just center the crosshair
        )))
    (:then_2
      ;;[0.3486 0.1284 1 0.7615] Distance To Objective Management
      (Utilities|IsValid _returnvalue_3
        (:Is%20Valid
          (bind _location_2 (Default|GetTargetableLocation _target)))
        (:Is%20Not%20Valid
          _))
      (Transformation|SetRelativeLocation (Variables|Default|GetCrosshairBetweenObjectiveOffset) (Math|Vector|Lerp(Vector) (Variables|/Script/Engine.SceneComponent|GetRelativeLocation (Variables|Default|GetCrosshairBetweenObjectiveOffset)) (* (+ (* (Math|Transform|InverseTransformLocation (Math|Transform|MakeTransform (.location _returnvalue_2) (.rotation _returnvalue_2) (.scale _returnvalue_2)) (select (Utilities|IsValid _returnvalue_3) _location_2 (.location _returnvalue_2))) (Variables|CrosshairEffectsConfig|GetProportionOfDistanceToEnemy)) (Variables|CrosshairEffectsConfig|GetBaseCrosshairOffset)) "1.000000, 0, 0") (Variables|CrosshairEffectsConfig|GetConvergenceRate)) false true))))

(fn ConstructionScript)