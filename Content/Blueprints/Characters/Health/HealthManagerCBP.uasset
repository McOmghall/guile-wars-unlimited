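; Health manager component that tracks an owning actor's health and reports damage and death through event dispatchers.
; On BeginPlay it fills health to maximum, and destroys the owner with a printed warning if that is zero or less.
; ReceiveDamage subtracts damage, broadcasts OnDamageReceived, then OnDie at zero or below, without destroying the owner.
; The WillDie value in both broadcasts is inverted, being true while health remains positive.
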(event EventBeginPlay
  (bind _output_get (Variables|Default|SetCurrentHealth (Variables|Default|GetMaxHealth)))
  (if (<= _output_get 0.0)
    (Development|PrintString "WARNING: Created actor with health 0 or less, destroying")
    (Actor|DestroyActor (Components|GetOwner))))

(fn ReceiveDamage
  (params (Damage :type Float%20%28single-precision%29))
  (bind _maxhealth (Variables|Default|GetMaxHealth))
  (bind _output_get (LocalVariables|SetHealthAfterDamage (+ (* Damage -1.0) (Variables|Default|GetCurrentHealth))))
  (Default|CallOnDamageReceived _maxhealth _output_get (> _output_get 0.0))
  (bind _output_get_2 (Variables|Default|SetCurrentHealth _output_get))
  (if (> _output_get 0.0)
    _
    (else
      (Default|CallOnDie _maxhealth _output_get_2 (> _output_get 0.0))))
  (return _output_get_2))